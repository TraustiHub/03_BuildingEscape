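; Openable door actor that swings open and closed in response to OnOpen and OnClose events from OpenDoor.
; It stores its starting rotation on BeginPlay, then the DoorSwing timeline adds an animated yaw to that rotation, playing forward to open and reversing to close.
; A Sound Timer event track on the same timeline plays the door sound at the actor's location, starting partway into the clip.
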(event OnClose(OpenDoor)
  (bind _openangle (Timeline|DoorSwing Reverse)
    (:Update
      (Transformation|SetActorRotation (Math|Rotator|CombineRotators (Math|Rotator|MakeRotator 0.0 0.0 _openangle) (Variables|Default|GetInitialRotation))))
    (:SoundTimer
      (Audio|PlaySoundatLocation "/Game/StarterContent/Audio/open_door_1.open_door_1" (Transformation|GetActorLocation) "0, 0, 0" 1.0 1.0 1.0))))

(event OnOpen(OpenDoor)
  (bind _openangle (Timeline|DoorSwing Play)
    (:Update
      (Transformation|SetActorRotation (Math|Rotator|CombineRotators (Math|Rotator|MakeRotator 0.0 0.0 _openangle) (Variables|Default|GetInitialRotation))))
    (:SoundTimer
      (Audio|PlaySoundatLocation "/Game/StarterContent/Audio/open_door_1.open_door_1" (Transformation|GetActorLocation) "0, 0, 0" 1.0 1.0 1.0))))

(event EventBeginPlay
  (Variables|Default|SetInitialRotation (Transformation|GetActorRotation)))

(fn ConstructionScript)